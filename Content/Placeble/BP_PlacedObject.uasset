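; Placeable product actor that displays a product asset's mesh on a scaled plate and supports moving, rotating and scaling.
; Construction applies mesh and plate size from BPProductAsset.
; Positioning line-traces from a deprojected screen point, snapping Scene to hits on BPPlane; the trace end omits the start position.
; Rotation yaws by inverted X input, while scaling takes small clamped steps following the sign of input change.
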(event EventBeginPlay)

(event Collision|EventActorBeginOverlap
  (params (OtherActor :type Actor%20Object%20Reference)))

(event EventTick
  (params (DeltaSeconds :type Float%20%28single-precision%29)))

(fn ConstructionScript
  (CallFunction|ASainProjectAssest))

(fn ASainProjectAssest
  (bind _bp_productasset (Variables|Default|GetBP_ProductAsset))
  (bind _platescale (Variables|/Game/Placeble/BP_ProductAsset.BP_ProductAsset_C|GetPlateScale _bp_productasset))
  (Components|StaticMesh|SetStaticMesh (Variables|Default|GetSM_Object) (Variables|/Game/Placeble/BP_ProductAsset.BP_ProductAsset_C|GetStaticMesh _bp_productasset))
  (Transformation|SetWorldScale3D (Variables|Default|GetSM_Plate) (Math|Vector|MakeVector _platescale _platescale 0.0)))

(fn SetPlacedPostion
  (params (Vector2D :type Vector%202D%20Structure))
  (bind _returnvalue (Game|GetPlayerController 0))
  (bind (_worldposition _worlddirection) (Class|GameplayStatics|DeprojectScreentoWorld _returnvalue Vector2D))
  (bind (_outhit _returnvalue_2) (Collision|LineTraceForObjects _worldposition (+ _worlddirection (* _worlddirection 1e+03)) (Utilities|Array|MakeArray "ObjectTypeQuery1" "ObjectTypeQuery2" "ObjectTypeQuery3" "ObjectTypeQuery4" "ObjectTypeQuery5" "ObjectTypeQuery6") false 0 "None"))
  (if _returnvalue_2
    (if (== (.HitActor (Collision|BreakHitResult _outhit)) (Variables|Default|GetBP_Plane))
      (Transformation|SetWorldLocation (Variables|Default|GetScene) (.Location (Collision|BreakHitResult _outhit)) false false))))

(fn SetPlacebleRotation
  (params (Dercetion :type Vector%202D%20Structure) (Location :type Vector%202D%20Structure))
  (Variables|Default|SetDestanceTrabled (+ (Math|Vector|Distance2D(Vector) Location (Variables|Default|GetPrebiusLocation)) (Variables|Default|GetDestanceTrabled)))
  (Variables|Default|SetPrebiusLocation Location)
  (Transformation|AddRelativeRotation (Variables|Default|GetScene) (Math|Rotator|MakeRotator 0.0 0.0 (* (.X (Math|Vector2D|BreakVector2D Dercetion)) -1.0)) false false))

(fn SetPlacebleScale
  (params (NewScaleMapping :type Float%20%28double-precision%29))
  (bind _output_get (Variables|Default|SetPre (Math|Float|Clamp(Float) (+ (* (Math|Float|Sign(Float) (- NewScaleMapping (Variables|Default|GetPreviusScaleMapping))) 0.01) (Variables|Default|GetPre)) 0.5 1.5)))
  (Transformation|SetWorldScale3D (Variables|Default|GetScene) (Math|Vector|MakeVector _output_get _output_get _output_get))
  (Variables|Default|SetPreviusScaleMapping NewScaleMapping))