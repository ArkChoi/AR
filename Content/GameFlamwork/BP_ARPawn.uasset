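; AR player pawn that creates the main menu and lets the player select a detected plane, then place and manipulate an object on it.
; After scanning, Tick periodically traces from screen center to refresh a BP_Plane candidate.
; Taps select the plane and spawn BP_PlacedObject on it.
; Timed touch detection locks one gesture until fingers lift: one finger moves, two fingers rotate or scale by drag direction.
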(event EventBeginPlay
  ;[0.15 0.15 0.15 0.5] Comment
  (bind _returnvalue (UserInterface|CreateWidget "/Game/UI/BP_MainMenu1.BP_MainMenu1_C" (Game|GetPlayerController 0)))
  (bind _output_get (Variables|Default|SetMainMenu _returnvalue))
  (UserInterface|Viewport|AddtoViewport _output_get 0))

(event EventTick
  (params (DeltaSeconds :type Float%20%28single-precision%29))
  (Variables|Default|SetDelta%20Seconds DeltaSeconds)
  (Utilities|FlowControl|Sequence
    (:then_0
      (CallFunction|ResetRecognisedJeture)
      (CallFunction|OnFingerJesthureNation)
      (CallFunction|TwoFingerJesthureNation)
      (if (Variables|Default|GetJesthureMecronised)
        (switch Utilities|FlowControl|Switch|SwitchonE_JesthureType (Variables|Default|GetCurrentTransformation)
          (:NewEnumerator0
            (Default|SetPlacedPostion (Variables|Default|GetPlacedObject) (CallFunction|GetTouchLocation)))
          (:NewEnumerator1
            (Default|SetPlacebleRotation (Variables|Default|GetPlacedObject) (CallFunction|GetFingderDilaction) (CallFunction|GetTouchLocation)))
          (:NewEnumerator2
            (Default|SetPlacebleScale (Variables|Default|GetPlacedObject) (Input|AxisValues|GetTwoFingerMapping))))))
    (:then_1
      (if (not (Variables|State|GetScaningIsDone))
        (Utilities|IsValid (Variables|Default|GetDepthTexter)
          (:Is%20Not%20Valid
            (bind _returnvalue (Class|ARBlueprintLibrary|GetARTexture "SceneDepthMap"))
            (Variables|Default|SetDepthTexter _returnvalue)))))
    (:then_2
      (if (and (Variables|State|GetScaningIsDone) (not (Variables|State|GetPalneIsSelected)))
        (bind _output_get (Variables|Default|SetShowPalneTimer (+ (Variables|Default|GetDelta%20Seconds) (Variables|Default|GetShowPalneTimer))))
        (if (> _output_get 1.0)
          (Variables|Default|SetShowPalneTimer 0.0)
          (CallFunction|UpdatePlaneCanDate))))))

(event Input|ActionEvents|InputActionOneFingerAction
  (params (Key :type Key%20Structure :default "None"))
  (:Pressed
    (bind _outhit (CallFunction|WorldHitTest (CallFunction|GetTouchLocation)))
    (Utilities|Casting|CastToBP_PlacedObject (.HitActor (Collision|BreakHitResult _outhit)))
    (Variables|Default|SetOneFingerPressed true)
    (Variables|Default|SetOneFingerValideTimer 0.0))
  (:Released
    (Variables|Default|SetOneFingerPressed false)))

(event Input|ActionEvents|InputActionTwoFingerAction
  (params (Key :type Key%20Structure :default "None"))
  (:Pressed
    (Variables|Default|SetTwoFingerPressed true)
    (Variables|Default|SetTwoFingerValideTimer 0.0)
    (bind _output_get (Variables|Default|SetPreviersFingerPosition (CallFunction|GetTouchLocation)))
    (Variables|Default|SetStartingFingerPosition _output_get)
    (Variables|Default|SetPreviusFinger%20Distance (CallFunction|GetFingerDistance)))
  (:Released
    (Variables|Default|SetTwoFingerPressed false)))

(event Input|TouchEvents|InputTouch
  (params (Location :type Vector) (FingerIndex :type ETouchIndex%20Enum))
  (:Pressed
    (switch Utilities|FlowControl|Switch|SwitchonETouchIndex FingerIndex
      (:Touch1
        (if (Variables|State|GetPalneIsSelected)
          (if (not (Variables|State|GetObjectIsPlaced))
            (bind (_outhit _returnvalue) (CallFunction|WorldHitTest (CallFunction|GetTouchLocation)))
            (if _returnvalue
              (if (== (.HitActor (Collision|BreakHitResult _outhit)) (Variables|Default|GetSelectedPlane))
                (bind _returnvalue_2 (Game|SpawnActorfromClass "/Game/Placeble/BP_PlacedObject.BP_PlacedObject_C" (Math|Conversions|ToTransform(Vector) (.Location (Collision|BreakHitResult _outhit))) "Undefined" "MultiplyWithRoot" 0 0))
                (bind _output_get (Variables|Default|SetPlacedObject _returnvalue_2))
                (Variables|/Game/Placeble/BP_PlacedObject.BP_PlacedObject_C|SetBP_Plane _output_get (Variables|Default|GetSelectedPlane))
                (Variables|State|SetObjectIsPlaced true)
                (Default|Hidden (Variables|Default|GetSelectedPlane))
                (Default|CallARObjectSpawned))))
          (else
            (bind (_outhit_2 _returnvalue_3) (CallFunction|WorldHitTest (CallFunction|GetTouchLocation)))
            (if _returnvalue_3
              (bind _asbp_plane (Utilities|Casting|CastToBP_Plane (.HitActor (Collision|BreakHitResult _outhit_2))))
              (Utilities|IsValid (Variables|/Game/Placeble/BP_Plane.BP_Plane_C|GetPlane _asbp_plane)
                (:Is%20Valid
                  (bind _output_get_2 (Variables|Default|SetSelectedPlane _asbp_plane))
                  (Default|CallBPPlaneSelected _output_get_2)
                  (Variables|State|SetPalneIsSelected true))))))))))

(fn ConstructionScript)

(fn UpdatePlaneCanDate
  (bind _returnvalue (Class|ARBlueprintLibrary|LineTraceTrackedObjects (CallFunction|GetScerinScenterPosion) false false))
  (Math|Integer|CompareInt (Utilities|Array|Length _returnvalue)
    (:>
      (bind _asarplane_geometry (Utilities|Casting|CastToARPlaneGeometry (Class|ARTraceResultLibrary|GetTrackedGeometry (Utilities|Array|Get(acopy) _returnvalue))))
      (bind _returnvalue_2 (CallFunction|CreatePlayingCanDate _asarplane_geometry (Class|ARTraceResultLibrary|GetTrackedGeometry (Utilities|Array|Get(acopy) _returnvalue))))
      (Utilities|IsValid _returnvalue_2
        (:Is%20Valid
          (Utilities|FlowControl|Sequence
            (:then_0
              (Utilities|IsValid (Variables|Default|GetBP_PlaneCandate)
                (:Is%20Valid
                  (Actor|DestroyActor (Variables|Default|GetBP_PlaneCandate)))))
            (:then_1
              (Variables|Default|SetBP_PlaneCandate _returnvalue_2))))))))

(fn GetScerinScenterPosion
  (bind _returnvalue (Game|GetPlayerController 0))
  (bind (_sizex _sizey) (HUD|GetViewportSize _returnvalue))
  (return (* (Math|Vector2D|MakeVector2D (Math|Conversions|ToFloat(Integer) _sizex) (Math|Conversions|ToFloat(Integer) _sizey)) 0.5)))

(fn CreatePlayingCanDate
  (params (ARPlane :type AR%20Plane%20Geometry%20Object%20Reference) (ARTracked :type AR%20Tracked%20Geometry%20Object%20Reference))
  (bind _returnvalue (Class|ARPlaneGeometry|GetExtent ARPlane))
  (bind _returnvalue_2 (/ _returnvalue 5e+01))
  (bind (_x _y) (Math|Vector|BreakVector _returnvalue_2))
  (bind _returnvalue_3 (Game|SpawnActorfromClass "/Game/Placeble/BP_Plane.BP_Plane_C" (Class|ARTrackedGeometry|GetLocaltoWorldTransform ARPlane) "Undefined" "MultiplyWithRoot" 0 0))
  (Transformation|SetRelativeScale3D (Variables|/Game/Placeble/BP_Plane.BP_Plane_C|GetPlane _returnvalue_3) (Math|Vector|MakeVector _x _y 0.0))
  (return _returnvalue_3))

(fn GetTouchLocation
  (bind _returnvalue (Game|GetPlayerController 0))
  (bind (_locationx _locationy) (Class|PlayerController|GetInputTouchState _returnvalue "Touch1"))
  (return (Math|Vector2D|MakeVector2D _locationx _locationy)))

(fn WorldHitTest
  (params (TouchLocation :type Vector%202D%20Structure))
  (bind _returnvalue (Game|GetPlayerController 0))
  (bind (_worldposition _worlddirection) (Class|GameplayStatics|DeprojectScreentoWorld _returnvalue TouchLocation))
  (bind (_outhit _returnvalue_2) (Collision|LineTraceForObjects _worldposition (+ _worlddirection (* _worlddirection 1e+03)) (Utilities|Array|MakeArray "ObjectTypeQuery1" "ObjectTypeQuery2" "ObjectTypeQuery3" "ObjectTypeQuery4" "ObjectTypeQuery5" "ObjectTypeQuery6") false 0 "None"))
  (return _outhit _returnvalue_2))

(fn ResetPlaceMent
  (bind _placedobject (Variables|Default|GetPlacedObject))
  (bind _selectedplane (Variables|Default|GetSelectedPlane))
  (Variables|State|SetObjectIsPlaced false)
  (Variables|State|SetPalneIsSelected false)
  (Utilities|FlowControl|Sequence
    (:then_0
      (Utilities|IsValid _placedobject
        (:Is%20Valid
          (Actor|DestroyActor _placedobject))))
    (:then_1
      (Utilities|IsValid _selectedplane
        (:Is%20Valid
          (Actor|DestroyActor _selectedplane))))))

(fn OnFingerJesthureNation
  (if (Math|Boolean|ANDBoolean (Variables|State|GetObjectIsPlaced) (Variables|Default|GetOneFingerPressed) (not (Variables|Default|GetJesthureMecronised)) (not (Variables|Default|GetTwoFingerPressed)))
    (bind _output_get (Variables|Default|SetOneFingerValideTimer (+ (Variables|Default|GetDelta%20Seconds) (Variables|Default|GetOneFingerValideTimer))))
    (if (> _output_get 0.2)
      (Variables|Default|SetJesthureMecronised true)
      (Variables|Default|SetCurrentTransformation "NewEnumerator0"))
    (else
      (Variables|Default|SetOneFingerValideTimer 0.0))))

(fn ResetRecognisedJeture
  (if (Variables|Default|GetJesthureMecronised)
    (if (not (CallFunction|AnyTouthReceved))
      (bind _output_get (Variables|Default|SetJesthurResetTimer (+ (Variables|Default|GetDelta%20Seconds) (Variables|Default|GetJesthurResetTimer))))
      (if (> _output_get 0.1)
        (Variables|Default|SetJesthureMecronised false)
        (Variables|Default|SetJesthurResetTimer 0.0))
      (else
        (Variables|Default|SetJesthurResetTimer 0.0)))))

(fn AnyTouthReceved
  (bind _returnvalue (Game|GetPlayerController 0))
  (return (or (.bIsCurrentlyPressed (Class|PlayerController|GetInputTouchState _returnvalue "Touch1")) (.bIsCurrentlyPressed (Class|PlayerController|GetInputTouchState _returnvalue "Touch2")))))

(fn GetFingerDistance
  (bind _returnvalue (Game|GetPlayerController 0))
  (bind (_locationx _locationy) (Class|PlayerController|GetInputTouchState _returnvalue "Touch2"))
  (bind (_locationx_2 _locationy_2) (Class|PlayerController|GetInputTouchState _returnvalue "Touch1"))
  (return (Math|Vector|Distance2D(Vector) (Math|Vector2D|MakeVector2D _locationx_2 _locationy_2) (Math|Vector2D|MakeVector2D _locationx _locationy))))

(fn TwoFingerJesthureNation
  (if (Math|Boolean|ANDBoolean (Variables|State|GetObjectIsPlaced) (Variables|Default|GetTwoFingerPressed) (not (Variables|Default|GetJesthureMecronised)))
    (bind _output_get (Variables|Default|SetTwoFingerValideTimer (+ (Variables|Default|GetDelta%20Seconds) (Variables|Default|GetTwoFingerValideTimer))))
    (if (> _output_get 0.2)
      (if (Math|Float|NearlyEqual(Float) (Math|Float|Absolute(Float) (- (Variables|Default|GetPreviusFinger%20Distance) (CallFunction|GetFingerDistance))) 0.0 0.001)
        (Variables|Default|SetTwoFingerValideTimer 0.0)
        (else
          (Variables|Default|SetJesthureMecronised true)
          (if (< (Math|Float|Absolute(Float) (.Y (Math|Vector2D|BreakVector2D (CallFunction|GetFingderDilaction)))) 0.5)
            (Variables|Default|SetCurrentTransformation "NewEnumerator1")
            (else
              (Variables|Default|SetCurrentTransformation "NewEnumerator2"))))))
    (else
      (Variables|Default|SetTwoFingerValideTimer 0.0))))

(fn GetFingderDilaction
  (bind _returnvalue (Game|GetPlayerController 0))
  (bind (_locationx _locationy) (Class|PlayerController|GetInputTouchState _returnvalue "Touch1"))
  (return (Math|Vector2D|Normalize2D (- (Math|Vector2D|MakeVector2D _locationx _locationy) (Variables|Default|GetPreviersFingerPosition)))))